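; Chess board actor that builds the board and sets up both teams on BeginPlay, starting with White's turn.
; It spawns a grid of tile actors, then fills a flat ChessPieces array indexed X*8+Y with team-colored piece prefabs and filler middle entries.
; Positioning moves pieces to computed tile centers, rotates one team 180 degrees and replaces each array entry with a newly added ChessPiece component.
; Tile highlighting functions are empty stubs.
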(event EventBeginPlay
  (Variables|Default|SetisWhiteTurn true)
  (CallFunction|GenerateAllTiles (Variables|Default|GetTILE_SIZE) (Variables|Default|GetTILE_COUNT_X) (Variables|Default|GetTILE_COUNT_Y))
  (CallFunction|SpawnAllPieces)
  (CallFunction|PositionAllPieces))

(event EventTick
  (params (DeltaSeconds :type Float%20%28single-precision%29)))

(fn GenerateAllTiles
  (params (tileSize :type Float%20%28double-precision%29) (tileCountX :type Integer) (tileCountY :type Integer))
  (Utilities|FlowControl|Sequence
    (:then_0
      ;[0 0.09551 0.162] Tiles is Cleared
      (Utilities|Array|Clear (Variables|Default|Gettiles)))
    (:then_1
      ;[0.03805 0.1683 0.01139] Zoffset
      (Variables|Default|SetzOffset (+ (Variables|Default|GetzOffset) (.Z (Math|Vector|BreakVector (Transformation|GetActorLocation (Variables|Default|GetPropertiesOfBoard)))))))
    (:then_2
      ;[0.2502 0.1735 0.01433] Bounds is set
      (Variables|Default|Setbounds (+ (Math|Vector|MakeVector (* (/ tileCountX 2) tileSize) (* (/ tileCountY 2) tileSize) 0.0) (Variables|Default|GetboardCentre))))
    (:then_3
      ;[0.2582 0.2623 0.2582] Tiles is set
      (for _index (range 0 (- tileCountX 1))
        (bind _output_get (LocalVariables|Setx _index))
        (for _index_2 (range 0 (- tileCountY 1))
          (bind _output_get_2 (LocalVariables|Sety _index_2))
          (bind _tileobject (CallFunction|GenerateSingleTile tileSize _output_get _output_get_2))
          (Utilities|Array|Add (Variables|Default|Gettiles) _tileobject))))))

(fn GenerateSingleTile
  (params (tileSize :type Float%20%28double-precision%29) (x :type Integer) (y :type Integer))
  ;[0.9911 0.1714 0] Spawning Tiles
  (bind _returnvalue (Game|SpawnActorfromClass "/Game/BluePrints/SpawnedTiles.SpawnedTiles_C" (Math|Conversions|ToTransform(Vector) (Math|Vector|MakeVector (+ (* x tileSize) -353.0) (+ (* y tileSize) -353.0) (Variables|Default|GetzOffset))) "Undefined" "MultiplyWithRoot" 0 0))
  (Variables|Default|SetTile%20Object _returnvalue)
  (Rendering|Material|SetMaterial (Variables|/Game/BluePrints/SpawnedTiles.SpawnedTiles_C|GetPlane _returnvalue) 0 (Variables|Default|GettileMaterial))
  (return (Variables|Default|GetTile%20Object)))

(fn SpawnAllPieces
  (bind _whiteteam (LocalVariables|GetwhiteTeam))
  (bind _blackteam (LocalVariables|GetblackTeam))
  (Utilities|Array|Clear (Variables|Default|GetchessPieces))
  (Utilities|FlowControl|Sequence
    (:then_0
      ;[1 1 1] White Team
      (Utilities|FlowControl|Sequence
        (:then_0
          (bind _cp (CallFunction|SpawnSinglePiece "NewEnumerator2" _whiteteam))
          (Variables|Default|SetchessPieces (Utilities|Array|MakeArray _cp)))
        (:then_1
          (bind _cp_2 (CallFunction|SpawnSinglePiece "NewEnumerator3" _whiteteam))
          (Utilities|Array|Insert (Variables|Default|GetchessPieces) _cp_2 1))
        (:then_2
          (bind _cp_3 (CallFunction|SpawnSinglePiece "NewEnumerator4" _whiteteam))
          (Utilities|Array|Insert (Variables|Default|GetchessPieces) _cp_3 2))
        (:then_3
          (bind _cp_4 (CallFunction|SpawnSinglePiece "NewEnumerator5" _whiteteam))
          (Utilities|Array|Insert (Variables|Default|GetchessPieces) _cp_4 3))
        (:then_4
          (bind _cp_5 (CallFunction|SpawnSinglePiece "NewEnumerator6" _whiteteam))
          (Utilities|Array|Insert (Variables|Default|GetchessPieces) _cp_5 4))
        (:then_5
          (bind _cp_6 (CallFunction|SpawnSinglePiece "NewEnumerator4" _whiteteam))
          (Utilities|Array|Insert (Variables|Default|GetchessPieces) _cp_6 5))
        (:then_6
          (bind _cp_7 (CallFunction|SpawnSinglePiece "NewEnumerator3" _whiteteam))
          (Utilities|Array|Insert (Variables|Default|GetchessPieces) _cp_7 6))
        (:then_7
          (bind _cp_8 (CallFunction|SpawnSinglePiece "NewEnumerator2" _whiteteam))
          (Utilities|Array|Insert (Variables|Default|GetchessPieces) _cp_8 7))
        (:then_8
          (for _index (range 8 15)
            (bind _cp_9 (CallFunction|SpawnSinglePiece "NewEnumerator1" _whiteteam))
            (Utilities|Array|Insert (Variables|Default|GetchessPieces) _cp_9 _index)))))
    (:then_1
      ;[0.5365 0 0] NONE
      (for _index_2 (range 16 47)
        (bind _cp_10 (CallFunction|SpawnSinglePiece "NewEnumerator8" -1))
        (Utilities|Array|Insert (Variables|Default|GetchessPieces) _cp_10 _index_2)))
    (:then_2
      ;[0 0 0] Black Team
      (Utilities|FlowControl|Sequence
        (:then_0
          (for _index_3 (range 48 55)
            (bind _cp_11 (CallFunction|SpawnSinglePiece "NewEnumerator1" _blackteam))
            (Utilities|Array|Insert (Variables|Default|GetchessPieces) _cp_11 _index_3)))
        (:then_1
          (bind _cp_12 (CallFunction|SpawnSinglePiece "NewEnumerator2" _blackteam))
          (Utilities|Array|Insert (Variables|Default|GetchessPieces) _cp_12 56))
        (:then_2
          (bind _cp_13 (CallFunction|SpawnSinglePiece "NewEnumerator3" _blackteam))
          (Utilities|Array|Insert (Variables|Default|GetchessPieces) _cp_13 57))
        (:then_3
          (bind _cp_14 (CallFunction|SpawnSinglePiece "NewEnumerator4" _blackteam))
          (Utilities|Array|Insert (Variables|Default|GetchessPieces) _cp_14 58))
        (:then_4
          (bind _cp_15 (CallFunction|SpawnSinglePiece "NewEnumerator5" _blackteam))
          (Utilities|Array|Insert (Variables|Default|GetchessPieces) _cp_15 59))
        (:then_5
          (bind _cp_16 (CallFunction|SpawnSinglePiece "NewEnumerator6" _blackteam))
          (Utilities|Array|Insert (Variables|Default|GetchessPieces) _cp_16 60))
        (:then_6
          (bind _cp_17 (CallFunction|SpawnSinglePiece "NewEnumerator4" _blackteam))
          (Utilities|Array|Insert (Variables|Default|GetchessPieces) _cp_17 61))
        (:then_7
          (bind _cp_18 (CallFunction|SpawnSinglePiece "NewEnumerator3" _blackteam))
          (Utilities|Array|Insert (Variables|Default|GetchessPieces) _cp_18 62))
        (:then_8
          (bind _cp_19 (CallFunction|SpawnSinglePiece "NewEnumerator2" _blackteam))
          (Utilities|Array|Insert (Variables|Default|GetchessPieces) _cp_19 63))))))

(fn SpawnSinglePiece
  (params (type :type ChessPieceType%20Enum :default "NewEnumerator8") (team :type Integer))
  (bind _returnvalue (Math|Conversions|ToInteger(Byte) type))
  (if (== _returnvalue 0)
    (return 0)
    (else
      (bind _returnvalue_2 (Game|SpawnActorfromClass (Utilities|Array|Get(acopy) (Variables|Default|Getprefabs) (- _returnvalue 1)) (Math|Transform|MakeTransform "0, 0, 0") "Undefined" "MultiplyWithRoot" 0 0))
      (LocalVariables|SetTempActor _returnvalue_2)
      (Class|BIChangeableMaterial|SetMaterialonActoors(Message) _returnvalue_2 (Utilities|Array|Get(acopy) (Variables|Default|GetteamMaterials) team))
      (bind _returnvalue_3 (Game|AddComponentbyClass _returnvalue_2 "/Game/BluePrints/ChessPiece.ChessPiece_C" type team 0 0 "0.000000,0.000000,0.000000" "1.000000,1.000000,1.000000" _returnvalue_2))
      (bind _output_get (Variables|Default|SetCp _returnvalue_3))
      (return _output_get))))

(fn PositionAllPieces
  (for _index (range 0 (- (Variables|Default|GetTILE_COUNT_X) 1))
    (bind _output_get (LocalVariables|Setx _index))
    (for _index_2 (range 0 (- (Variables|Default|GetTILE_COUNT_Y) 1))
      (bind _output_get_2 (LocalVariables|Sety _index_2))
      (bind _output_get_3 (LocalVariables|Setindex (+ (* _output_get 8) 0)))
      (if (and (!= 0 (Math|Conversions|ToInteger(Byte) (Variables|/Game/BluePrints/ChessPiece.ChessPiece_C|Gettype (Utilities|Array|Get(acopy) (Variables|Default|GetchessPieces) _output_get_3)))) (Utilities|IsValid (Utilities|Array|Get(acopy) (Variables|Default|GetchessPieces) _output_get_3)))
        (CallFunction|PositionSinglePiece _output_get _output_get_2 true)))))

(fn PositionSinglePiece
  (params (x :type Integer) (y :type Integer) (force :type Boolean))
  (bind _output_get (LocalVariables|Setindex (+ (* x 8) y)))
  (bind _tilecenterreturn (CallFunction|GetTileCenter x y))
  (if (== (Variables|/Game/BluePrints/ChessPiece.ChessPiece_C|Getteam (Utilities|Array|Get(acopy) (Variables|Default|GetchessPieces) _output_get)) 0)
    (LocalVariables|SetTempZrotator 1.8e+02)
    (else
      (LocalVariables|SetTempZrotator 0.0)))
  (Class|Actor|AddActorWorldTransform (Variables|/Game/BluePrints/ChessPiece.ChessPiece_C|GetCPType (Utilities|Array|Get(acopy) (Variables|Default|GetchessPieces) _output_get)) (Math|Transform|MakeTransform _tilecenterreturn (Math|Rotator|MakeRotator 0.0 0.0 (LocalVariables|GetTempZrotator)) "1.000000,1.000000,1.000000") false false)
  (bind _returnvalue (Game|AddComponentbyClass (Variables|/Game/BluePrints/ChessPiece.ChessPiece_C|GetCPType (Utilities|Array|Get(acopy) (Variables|Default|GetchessPieces) _output_get)) "/Game/BluePrints/ChessPiece.ChessPiece_C" (Variables|/Game/BluePrints/ChessPiece.ChessPiece_C|Gettype (Utilities|Array|Get(acopy) (Variables|Default|GetchessPieces) _output_get)) (Variables|/Game/BluePrints/ChessPiece.ChessPiece_C|Getteam (Utilities|Array|Get(acopy) (Variables|Default|GetchessPieces) _output_get)) x y _tilecenterreturn "1.000000,1.000000,1.000000" (Variables|/Game/BluePrints/ChessPiece.ChessPiece_C|GetCPType (Utilities|Array|Get(acopy) (Variables|Default|GetchessPieces) _output_get))))
  (Utilities|Array|SetArrayElem (Variables|Default|GetchessPieces) _output_get _returnvalue))

(fn GetTileCenter
  (params (x :type Integer) (y :type Integer))
  (bind _tile_size (Variables|Default|GetTILE_SIZE))
  (bind _tile_size_2 (Variables|Default|GetTILE_SIZE))
  (bind _output_get (LocalVariables|SetV3D (Math|Vector|MakeVector (* x _tile_size) (* y _tile_size) (Variables|Default|GetzOffset))))
  (bind _output_get_2 (LocalVariables|SetV3D (+ (- _output_get (Variables|Default|Getbounds)) (Math|Vector|MakeVector (/ _tile_size_2 2.0) (/ _tile_size_2 2.0) 0.0))))
  (return _output_get_2))

(fn HighLightTiles
  (for _index (range 0 (- (Utilities|Array|Length (Variables|Default|GetavailableMoves)) 1))
    _))

(fn RemoveHighlightTiles)

(fn SetChessPieceVariables
  (params (type_enum :type ChessPieceType%20Enum%20%28by%20ref%29 :default "NewEnumerator8") (team_int :type Integer%20%28by%20ref%29) (cp_actor :type Actor%20Object%20Reference%20%28by%20ref%29))
  (return 0))

(fn SetMaterialonActoors
  (params (Mat :type Material%20Object%20Reference)))